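; Passive effect Blueprint for the character Saiqi, driving combat reactions through battle events, buffs and skill effects.
; Entering the ultimate adds grade-gated buffs (2/4/6), and draining SP switches it off.
; Crits grant random buffs, ranged hits detonate mark stacks, and grade-2 missiles can spawn phantoms via the client effect.
; Damage scales with capped buff count, with extra handlers for grab hits and the flying skill's missile origin.
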(event SpChanged(BattleEvent)
  (params (Character :type Character%20Base%20Object%20Reference) (Before :type Integer%20%28by%20ref%29) (After :type Integer%20%28by%20ref%29) (Reason :type EChangedSpReason%20Enum :default "FromBP"))
  ;[1 1 1] 0SP解除大招
  (if (and (>= Before After) (< After 1))
    (bind _returnvalue (Class|Battle|CheckConditionNew (CallFunction|Battle) 530123 Character 0 (Utilities|Name|MakeLiteralName "From BP_Saiqi:SpChanged")))
    (if _returnvalue
      (CallFunction|Skill2Off Character 530102 530121 (Utilities|Array|MakeArray 530122)))))

(event InitDamageLow(BattleEvent)
  (params (Character :type Character%20Base%20Object%20Reference) (Damage :type Damage%20Struct%20Object%20Reference) (Source :type Effect%20Source%20Interface%20Interface%20%28by%20ref%29) (Target :type Effect%20Source%20Interface%20Interface%20%28by%20ref%29))
  (bind _passiveowner (Variables|Default|GetPassiveOwner))
  (bind _passiveowner_2 (Variables|Default|GetPassiveOwner))
  (bind _passiveowner_3 (Variables|Default|GetPassiveOwner))
  (bind _returnvalue (Class|CharacterFunctionLibrary|CasttoCharacterBase _passiveowner))
  (bind _returnvalue_2 (Class|CharacterFunctionLibrary|CasttoCharacterBase _passiveowner_2))
  (bind _returnvalue_3 (Class|CharacterBase|GetSkill _returnvalue 530111))
  (bind _returnvalue_4 (Class|CharacterBase|GetSkill _returnvalue_2 530111))
  (Utilities|FlowControl|Sequence
    (:then_0
      ;[1 1 1] 触发暴击时，为赛琪附加【攻击提升/技能强度提升/背水】其中一个随机增益，持续T秒。
      (if (Class|DamageStruct|IsDamageCrit Damage)
        (Class|BattleFunctionLibrary|AddBufftoTarget _passiveowner_3 _passiveowner_3 (+ (Math|Random|RandomInteger 3) 530131) (Variables|Default|GetPassiveBuffLastTime) 0.0 self)))
    (:then_1
      ;[1 1 1] 射击时引爆1层印记
      (if (Class|DamageStruct|HaveDamageTag Damage (Utilities|Name|MakeLiteralName "Ranged"))
        (bind _returnvalue_5 (Class|BattleFunctionLibrary|ReduceBuffLayerfromTarget _passiveowner Target 530102 1 true))
        (if _returnvalue_5
          (Class|BattleFunctionLibrary|ExecuteSkillEffects _passiveowner (Utilities|Array|MakeArray 530116) Target _returnvalue_3 _returnvalue_3 0) ; 引爆伤害
        )))
    (:then_2
      ;[1 1 1] 2命效果，导弹命中生成幻象
      (if (CallFunction|CheckSkillGrade (Variables|Default|GetOwnerSkill) 2)
        (if (Class|DamageStruct|HaveDamageTag Damage (Utilities|String|StringToName (Utilities|String|MakeLiteralString "SaiqiSkill01")))
          (if (CallFunction|概率执行 (Variables|Default|GetGrade2TriggerProb))
            (Default|Skill1SnapShot (.AsBP%20Saiqi%20Client (Utilities|Casting|CastToBP_Saiqi_Client (Variables|Default|GetPassiveEffectClient))))
            (Class|BattleFunctionLibrary|ExecuteSkillEffects _passiveowner_2 (Utilities|Array|MakeArray 530117) Target _returnvalue_4 _returnvalue_4 0) ; 引爆伤害
          ))))))

(event OnBeforeGrabHit(BattleEvent)
  (params (Character :type Character%20Base%20Object%20Reference))
  (bind _passiveowner (Variables|Default|GetPassiveOwner))
  ;[1 1 1] 投技等特殊受击处理
  (Class|BattleFunctionLibrary|ExecuteSkillEffects _passiveowner (Utilities|Array|MakeArray 530122) 0 0 (Class|CharacterFunctionLibrary|CasttoCharacterBase _passiveowner) 0))

(event EnterNode(BattleEvent)
  (params (Character :type Character%20Base%20Object%20Reference) (NodeId :type Integer%20%28by%20ref%29) (SkillNode :type Skill%20Node%20Object%20Reference))
  (bind _skill (Variables|/Script/EM.SkillNode|GetSkill SkillNode))
  (bind _passiveowner (Variables|Default|GetPassiveOwner))
  ;[1 1 1] 2命-自动飞弹
  (if (== NodeId 530121)
    (if (CallFunction|CheckSkillGrade _skill 2)
      (Class|BattleFunctionLibrary|AddBufftoTarget _passiveowner _passiveowner 530122 -1.0 0.0)
      ;[1 1 1] 4命：开大期间额外获得霸体+减伤
      (if (CallFunction|CheckSkillGrade _skill 4)
        (Class|BattleFunctionLibrary|AddBufftoTarget _passiveowner _passiveowner 530112 -1.0 0.0)
        ;[1 1 1] 6命：开大期间获得属性穿透（不是Buff）
        (if (CallFunction|CheckSkillGrade _skill 6)
          (Class|BattleFunctionLibrary|AddBufftoTarget _passiveowner _passiveowner 530113 -1.0 0.0))))))

(event InitDamage(BattleEvent)
  (params (Character :type Character%20Base%20Object%20Reference) (Damage :type Damage%20Struct%20Object%20Reference) (Source :type Effect%20Source%20Interface%20Interface%20%28by%20ref%29) (Target :type Effect%20Source%20Interface%20Interface%20%28by%20ref%29))
  (bind _passiveowner (Variables|Default|GetPassiveOwner))
  ;[1 1 1] 依据身上的增益效果数量，每个增益效果提升X%造成伤害，最多叠加N次。
  (Class|DamageStruct|AddGlobalDamageRate Damage (+ 1.0 (* (Math|Integer|Min(Integer) (+ (Utilities|Array|Length (Class|BattleFunctionLibrary|FindBuffsbyBuffType _passiveowner 10 0 false)) (Utilities|Array|Length (Class|BattleFunctionLibrary|FindBuffsbyBuffType _passiveowner 11 0 false))) (Variables|Default|GetMaxBuffCount)) (Variables|Default|GetPassiveDmgRate))) "Normal" false))

(event Custom|FlyingSkill1
  (bind _passiveowner (Variables|Default|GetPassiveOwner))
  (bind _returnvalue (Class|CharacterFunctionLibrary|CasttoCharacterBase _passiveowner))
  (bind _returnvalue_2 (Class|CharacterBase|GetSkill _returnvalue 530111))
  ;[1 1 1] 飞行E技能
  (Class|DataSetFunctionLibrary|SetSaveLoc _returnvalue (Transformation|GetSocketLocation (Variables|/Script/Engine.Character|GetMesh _returnvalue) "spine_03_decorate") "SaiqiMissle")
  (Class|BattleFunctionLibrary|ExecuteSkillEffects _passiveowner (Utilities|Array|MakeArray 530112 530118) _passiveowner _returnvalue_2 _returnvalue_2 0))

(fn ConstructionScript)